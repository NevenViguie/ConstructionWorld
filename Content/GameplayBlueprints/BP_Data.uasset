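; BP_Data is a quiz data holder that stores difficulty, the current question and counts of right and wrong answers behind getters and setters.
; SetupQuestions fills an index list sized from the Questions column of DT_Questions, removes the hardcoded value 13, then shuffles it.
; SetCurrentQuestion increments a question counter and uses it to pick the current question index from that shuffled list.
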(fn `GetCurrentQuestion`
  (returns (CurrentQuestion :type Integer))
  (return (`self.CurrentQuestion`)))

(fn `GetDifficulty`
  (returns (Difficulty :type String))
  (return (`self.Difficulty`)))

(fn `GetRightAnswers`
  (returns (RightAnswers :type Integer))
  (return (`self.NumberOfRightAnswers`)))

(fn `GetWrongAnswers`
  (returns (WrongAnswers :type Integer))
  (return (`self.NumberOfWrongAnswers`)))

(fn `SetCurrentQuestion`
  (params (CurrentQuestion :type Integer) (CurrentPhase :type Integer))
  (returns (NewQuestion :type Integer))
  (bind _result (`/Engine/EditorBlueprintResources/StandardMacros.IncrementInt` CurrentQuestion)
    (:`  `
      (bind _output_get (set `self.CurrentQuestion` (`|GetArrayItem` (`self.Questions`) _result)))
      (return _output_get))))

(fn `SetDifficulty`
  (params (Difficulty :type String))
  (set `self.Difficulty` Difficulty))

(fn `SetRightAnswers`
  (params (RightAnswers :type Integer))
  (set `self.NumberOfRightAnswers` RightAnswers))

(fn `SetupQuestions`
  (bind _questions (`self.Questions`))
  (bind _returnvalue (`DataTableFunctionLibrary.GetDataTableColumnAsString` "/Game/GameplayBlueprints/Cards/DT_Questions.DT_Questions" "Questions"))
  (for _index (range (+ (`KismetArrayLibrary.Array_Length` _returnvalue) 1))
    (`KismetArrayLibrary.Array_Add` _questions _index))
  (`KismetArrayLibrary.Array_RemoveItem` _questions 13)
  (`KismetArrayLibrary.Array_Shuffle` (`self.Questions`)))

(fn `SetWrongAnswers`
  (params (WrongAnswers :type Integer))
  (set `self.NumberOfWrongAnswers` WrongAnswers))