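; BP_Building is a building that visually appears in stages through an "Appearance" scalar parameter on its static mesh materials.
; BeginPlay applies a hardcoded starting progression to the materials.
; Each ProgressBuilding call plays the Alpha timeline to blend the parameter up by a small fixed step, then saves the new progression when finished.
; A second timeline driving the same parameter is left unconnected.
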(event `self.ReceiveBeginPlay`
  (bind _output_get (set `self.CurrentProgression` 0.532))
  (`MeshComponent.SetScalarParameterValueOnMaterials` (`self.StaticMesh`) "Appearance" _output_get))

(event `ProgressBuilding`
  (bind _currentprogression (`self.CurrentProgression`))
  (bind _returnvalue (+ _currentprogression 0.0233))
  (bind (_direction _alpha) (`Timeline|Alpha` :!via `PlayFromStart`)
    (:`Update`
      (`MeshComponent.SetScalarParameterValueOnMaterials` (`self.StaticMesh`) "Appearance" (`KismetMathLibrary.Lerp` _currentprogression _returnvalue _alpha)))
    (:`Finished`
      (set `self.CurrentProgression` _returnvalue))))

(fn `UserConstructionScript`)