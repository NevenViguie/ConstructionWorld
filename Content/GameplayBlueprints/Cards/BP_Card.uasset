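; BP_Card runs a phased quiz through a four-button widget, where each correct answer advances a Building.
; Clicks update right/wrong tallies in GI_Data, flash the answer's color, then load the next question, switching phase DataTable every six questions.
; NewCard treats "Réponse 1" as correct and randomizes its slot among two Easy or four Hard choices.
; A Delay on Tick drives the on-screen minutes/seconds timer.
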(event `OnClicked_Btn1`
  (bind _gi_data (`self.GI_Data`))
  (bind _gi_data_2 (`self.GI_Data`))
  ;[1 0.3459 0.1795] Button 1
  (`/Game/GameplayBlueprints/Cards/WBP_Card.StopInput` (`self.WidgetRef`))
  (if (== (`self.RightAnswerIndex`) 0)
    (bind _rightanswers (`/Game/GameplayBlueprints/GI_Data.GetRightAnswers` _gi_data))
    (bind _result (`/Engine/EditorBlueprintResources/StandardMacros.IncrementInt` _rightanswers)
      (:`  `
        (`/Game/GameplayBlueprints/GI_Data.SetRightAnswers` _gi_data _result)
        (`TextBlock.SetColorAndOpacity` (`/Game/GameplayBlueprints/Cards/WBP_Card.Reponse1` (`self.WidgetRef`)) (make `SlateColor` (`self.ColorTrue`)))
        (`KismetSystemLibrary.Delay` 1.0)
        (`TextBlock.SetColorAndOpacity` (`/Game/GameplayBlueprints/Cards/WBP_Card.Reponse1` (`self.WidgetRef`)) (make `SlateColor` (`self.ColorBaseText`)))
        (`/Game/GameplayBlueprints/Building/BP_Building.ProgressBuilding` (`self.Building`))))
    (else
      (bind _wronganswers (`/Game/GameplayBlueprints/GI_Data.GetWrongAnswers` _gi_data_2))
      (bind _result_2 (`/Engine/EditorBlueprintResources/StandardMacros.IncrementInt` _wronganswers)
        (:`  `
          (`/Game/GameplayBlueprints/GI_Data.SetWrongAnswers` _gi_data_2 _result_2)
          (`TextBlock.SetColorAndOpacity` (`/Game/GameplayBlueprints/Cards/WBP_Card.Reponse1` (`self.WidgetRef`)) (make `SlateColor` (`self.ColorFalse`)))
          (`KismetSystemLibrary.Delay` 1.0)
          (`TextBlock.SetColorAndOpacity` (`/Game/GameplayBlueprints/Cards/WBP_Card.Reponse1` (`self.WidgetRef`)) (make `SlateColor` (`self.ColorBaseText`)))))))
  ;[1 1 1] Phases & New question
  (bind _result_3 (`/Engine/EditorBlueprintResources/StandardMacros.IncrementInt` (`self.QuestionIndex`) :!label _label)
    (:`  `
      (bind _output_get (set `self.QuestionIndex` _result_3))
      (if (> _output_get 5)
        (bind _result_4 (`/Engine/EditorBlueprintResources/StandardMacros.IncrementInt` (`self.Current Phase`))
          (:`  `
            (set `self.Current Phase` _result_4)
            (set `self.QuestionIndex` 0)
            (bind _newquestion (`/Game/GameplayBlueprints/GI_Data.SetCurrentQuestion` (`self.GI_Data`) 0 (`self.Current Phase`)))
            (set `self.CurrentQuestion` _newquestion)
            (set `self.Data Table` (select `int` (`self.Current Phase`) :`0` "/Game/GameplayBlueprints/Cards/Data/DT_Phase1.DT_Phase1" :`1` "/Game/GameplayBlueprints/Cards/Data/DT_Phase2.DT_Phase2" :`2` "/Game/GameplayBlueprints/Cards/Data/DT_Phase3.DT_Phase3" :!type "DataTable Object Reference"))))
        (else
          (bind _newquestion_2 (`/Game/GameplayBlueprints/GI_Data.SetCurrentQuestion` (`self.GI_Data`) (`self.QuestionIndex`) (`self.Current Phase`)))
          (set `self.CurrentQuestion` _newquestion_2)))
      (`self.NewCard`))))

(event `OnClicked_Btn2`
  (bind _gi_data (`self.GI_Data`))
  (bind _gi_data_2 (`self.GI_Data`))
  ;[1 0.3459 0.1795] Button 2
  (`/Game/GameplayBlueprints/Cards/WBP_Card.StopInput` (`self.WidgetRef`))
  (if (== (`self.RightAnswerIndex`) 1)
    (bind _rightanswers (`/Game/GameplayBlueprints/GI_Data.GetRightAnswers` _gi_data))
    (bind _result (`/Engine/EditorBlueprintResources/StandardMacros.IncrementInt` _rightanswers)
      (:`  `
        (`/Game/GameplayBlueprints/GI_Data.SetRightAnswers` _gi_data _result)
        (`TextBlock.SetColorAndOpacity` (`/Game/GameplayBlueprints/Cards/WBP_Card.Reponse2` (`self.WidgetRef`)) (make `SlateColor` (`self.ColorTrue`)))
        (`KismetSystemLibrary.Delay` 1.0)
        (`TextBlock.SetColorAndOpacity` (`/Game/GameplayBlueprints/Cards/WBP_Card.Reponse2` (`self.WidgetRef`)) (make `SlateColor` (`self.ColorBaseText`)))
        (`/Game/GameplayBlueprints/Building/BP_Building.ProgressBuilding` (`self.Building`))
        (goto _label)))
    (else
      (bind _wronganswers (`/Game/GameplayBlueprints/GI_Data.GetWrongAnswers` _gi_data_2))
      (bind _result_2 (`/Engine/EditorBlueprintResources/StandardMacros.IncrementInt` _wronganswers)
        (:`  `
          (`/Game/GameplayBlueprints/GI_Data.SetWrongAnswers` _gi_data_2 _result_2)
          (`TextBlock.SetColorAndOpacity` (`/Game/GameplayBlueprints/Cards/WBP_Card.Reponse2` (`self.WidgetRef`)) (make `SlateColor` (`self.ColorFalse`)))
          (`KismetSystemLibrary.Delay` 1.0)
          (`TextBlock.SetColorAndOpacity` (`/Game/GameplayBlueprints/Cards/WBP_Card.Reponse2` (`self.WidgetRef`)) (make `SlateColor` (`self.ColorBaseText`)))
          (goto _label))))))

(event `self.ReceiveBeginPlay`
  ;[0.2894 0.3569 1] Setup
  (`|ExecutionSequence`
    (:`then_0`
      (bind _asgi_data (cast `/Game/GameplayBlueprints/GI_Data` (`GameplayStatics.GetGameInstance`)))
      (bind _output_get (set `self.GI_Data` _asgi_data))
      (`/Game/GameplayBlueprints/GI_Data.SetupQuestions` _output_get)
      (bind _currentquestion (`/Game/GameplayBlueprints/GI_Data.GetCurrentQuestion` (`self.GI_Data`)))
      (set `self.CurrentQuestion` _currentquestion))
    (:`then_1`
      (bind _returnvalue (`|GenericCreateObject` (`self.WidgetClassRef`)))
      (bind _output_get_2 (set `self.WidgetRef` _returnvalue))
      (set `/Game/GameplayBlueprints/Cards/WBP_Card.PhaseText` (`self.Phase Text`) _output_get_2)
      (`UserWidget.AddToViewport` (`self.WidgetRef`) 0)
      (`|ExecutionSequence`
        (:`then_0`
          ;[1 0.3459 0.1795] Button 1
          (add `Button.OnClicked` (`/Game/GameplayBlueprints/Cards/WBP_Card.Button1` (`self.WidgetRef`)) (delegate `OnClicked_Btn1`)))
        (:`then_1`
          ;[1 0.3459 0.1795] Button 2
          (add `Button.OnClicked` (`/Game/GameplayBlueprints/Cards/WBP_Card.Button2` (`self.WidgetRef`)) (delegate `OnClicked_Btn2`)))
        (:`then_2`
          ;[1 0.3459 0.1795] Button 3
          (add `Button.OnClicked` (`/Game/GameplayBlueprints/Cards/WBP_Card.Button3` (`self.WidgetRef`)) (delegate `OnClicked_Btn3`)))
        (:`then_3`
          ;[1 0.3459 0.1795] Button 4
          (add `Button.OnClicked` (`/Game/GameplayBlueprints/Cards/WBP_Card.Button4` (`self.WidgetRef`)) (delegate `OnClicked_Btn4`)))))))

(event `OnClicked_Btn3`
  (bind _gi_data (`self.GI_Data`))
  (bind _gi_data_2 (`self.GI_Data`))
  ;[1 0.3459 0.1795] Button 3
  (`/Game/GameplayBlueprints/Cards/WBP_Card.StopInput` (`self.WidgetRef`))
  (if (== (`self.RightAnswerIndex`) 2)
    (bind _rightanswers (`/Game/GameplayBlueprints/GI_Data.GetRightAnswers` _gi_data))
    (bind _result (`/Engine/EditorBlueprintResources/StandardMacros.IncrementInt` _rightanswers)
      (:`  `
        (`/Game/GameplayBlueprints/GI_Data.SetRightAnswers` _gi_data _result)
        (`TextBlock.SetColorAndOpacity` (`/Game/GameplayBlueprints/Cards/WBP_Card.Reponse3` (`self.WidgetRef`)) (make `SlateColor` (`self.ColorTrue`)))
        (`KismetSystemLibrary.Delay` 1.0)
        (`TextBlock.SetColorAndOpacity` (`/Game/GameplayBlueprints/Cards/WBP_Card.Reponse3` (`self.WidgetRef`)) (make `SlateColor` (`self.ColorBaseText`)))
        (`/Game/GameplayBlueprints/Building/BP_Building.ProgressBuilding` (`self.Building`))
        (goto _label)))
    (else
      (bind _wronganswers (`/Game/GameplayBlueprints/GI_Data.GetWrongAnswers` _gi_data_2))
      (bind _result_2 (`/Engine/EditorBlueprintResources/StandardMacros.IncrementInt` _wronganswers)
        (:`  `
          (`/Game/GameplayBlueprints/GI_Data.SetWrongAnswers` _gi_data_2 _result_2)
          (`TextBlock.SetColorAndOpacity` (`/Game/GameplayBlueprints/Cards/WBP_Card.Reponse3` (`self.WidgetRef`)) (make `SlateColor` (`self.ColorFalse`)))
          (`KismetSystemLibrary.Delay` 1.0)
          (`TextBlock.SetColorAndOpacity` (`/Game/GameplayBlueprints/Cards/WBP_Card.Reponse3` (`self.WidgetRef`)) (make `SlateColor` (`self.ColorBaseText`)))
          (goto _label))))))

(event `SetDifficulty`
  (bind _widgetref (`self.WidgetRef`))
  (bind _widgetref_2 (`self.WidgetRef`))
  ;[1 0.4352 0.7684] Set difficulty
  (bind _difficulty (`/Game/GameplayBlueprints/GI_Data.GetDifficulty` (`self.GI_Data`)))
  (if (`KismetStringLibrary.EqualEqual_StrStr` _difficulty "Easy")
    (set `/Game/GameplayBlueprints/Cards/WBP_Card.Btn1Visibility` "Hidden" _widgetref)
    (set `/Game/GameplayBlueprints/Cards/WBP_Card.BtnBgndVisibility` "Hidden" _widgetref_2)
    (set `self.Difficulty` "Easy")
    (else
      (set `/Game/GameplayBlueprints/Cards/WBP_Card.Btn1Visibility` "Visible" _widgetref)
      (set `/Game/GameplayBlueprints/Cards/WBP_Card.BtnBgndVisibility` "HitTestInvisible" _widgetref_2)
      (set `self.Difficulty` "Hard"))))

(event `OnClicked_Btn4`
  (bind _gi_data (`self.GI_Data`))
  (bind _gi_data_2 (`self.GI_Data`))
  ;[1 0.3459 0.1795] Button 4
  (`/Game/GameplayBlueprints/Cards/WBP_Card.StopInput` (`self.WidgetRef`))
  (if (== (`self.RightAnswerIndex`) 3)
    (bind _rightanswers (`/Game/GameplayBlueprints/GI_Data.GetRightAnswers` _gi_data))
    (bind _result (`/Engine/EditorBlueprintResources/StandardMacros.IncrementInt` _rightanswers)
      (:`  `
        (`/Game/GameplayBlueprints/GI_Data.SetRightAnswers` _gi_data _result)
        (`TextBlock.SetColorAndOpacity` (`/Game/GameplayBlueprints/Cards/WBP_Card.Reponse4` (`self.WidgetRef`)) (make `SlateColor` (`self.ColorTrue`)))
        (`KismetSystemLibrary.Delay` 1.0)
        (`TextBlock.SetColorAndOpacity` (`/Game/GameplayBlueprints/Cards/WBP_Card.Reponse4` (`self.WidgetRef`)) (make `SlateColor` (`self.ColorBaseText`)))
        (`/Game/GameplayBlueprints/Building/BP_Building.ProgressBuilding` (`self.Building`))
        (goto _label)))
    (else
      (bind _wronganswers (`/Game/GameplayBlueprints/GI_Data.GetWrongAnswers` _gi_data_2))
      (bind _result_2 (`/Engine/EditorBlueprintResources/StandardMacros.IncrementInt` _wronganswers)
        (:`  `
          (`/Game/GameplayBlueprints/GI_Data.SetWrongAnswers` _gi_data_2 _result_2)
          (`TextBlock.SetColorAndOpacity` (`/Game/GameplayBlueprints/Cards/WBP_Card.Reponse4` (`self.WidgetRef`)) (make `SlateColor` (`self.ColorFalse`)))
          (`KismetSystemLibrary.Delay` 1.0)
          (`TextBlock.SetColorAndOpacity` (`/Game/GameplayBlueprints/Cards/WBP_Card.Reponse4` (`self.WidgetRef`)) (make `SlateColor` (`self.ColorBaseText`)))
          (goto _label))))))

(event `NewCard`
  (bind _widgetref (`self.WidgetRef`))
  (bind _widgetref_2 (`self.WidgetRef`))
  (bind _widgetref_3 (`self.WidgetRef`))
  (bind _answers (`self.Answers`))
  ;[1 1 1] New card
  (`/Game/GameplayBlueprints/Cards/WBP_Card.ResumeInput` (`self.WidgetRef`))
  (`|ExecutionSequence`
    (:`then_0`
      (bind _returnvalue (`DataTableFunctionLibrary.GetDataTableColumnAsString` (`self.Data Table`) "Phase"))
      (`/Game/GameplayBlueprints/Cards/WBP_Card.SetPhase` (`self.WidgetRef`) (`KismetTextLibrary.Conv_StringToText` (`|GetArrayItem` _returnvalue (`self.CurrentQuestion`)))))
    (:`then_1`
      (bind _returnvalue_2 (`DataTableFunctionLibrary.GetDataTableColumnAsString` (`self.Data Table`) "Questions"))
      (`/Game/GameplayBlueprints/Cards/WBP_Card.SetQuestion` (`self.WidgetRef`) (`KismetTextLibrary.Conv_StringToText` (`|GetArrayItem` _returnvalue_2 (`self.CurrentQuestion`)))))
    (:`then_2`
      (if (`KismetStringLibrary.EqualEqual_StrStr` (`self.Difficulty`) "Easy")
        (`|ExecutionSequence`
          (:`then_0`
            (bind _returnvalue_3 (`DataTableFunctionLibrary.GetDataTableColumnAsString` (`self.Data Table`) "Réponse 1"))
            (bind _output_get (set `self.Answer1` (`|GetArrayItem` _returnvalue_3 (`self.CurrentQuestion`))))
            (`KismetSystemLibrary.PrintString` _output_get)
            (bind _returnvalue_4 (`DataTableFunctionLibrary.GetDataTableColumnAsString` (`self.Data Table`) (select `int` (`KismetMathLibrary.RandomInteger` 3) :`0` "Réponse 2" :`1` "Réponse 3" :`2` "Réponse 4" :!type "Name")))
            (set `self.Answer2` (`|GetArrayItem` _returnvalue_4 (`self.CurrentQuestion`))))
          (:`then_1`
            (if (< (`KismetMathLibrary.RandomInteger` 2) 1)
              (set `/Game/GameplayBlueprints/Cards/WBP_Card.Reponse2_Text` (`KismetTextLibrary.Conv_StringToText` (`self.Answer1`)) _widgetref_2)
              (set `/Game/GameplayBlueprints/Cards/WBP_Card.Reponse3_Text` (`KismetTextLibrary.Conv_StringToText` (`self.Answer2`)) _widgetref_2)
              (set `self.RightAnswerIndex` 1)
              (else
                (set `/Game/GameplayBlueprints/Cards/WBP_Card.Reponse2_Text` (`KismetTextLibrary.Conv_StringToText` (`self.Answer2`)) _widgetref)
                (set `/Game/GameplayBlueprints/Cards/WBP_Card.Reponse3_Text` (`KismetTextLibrary.Conv_StringToText` (`self.Answer1`)) _widgetref)
                (set `self.RightAnswerIndex` 2)))))
        (else
          (`|ExecutionSequence`
            (:`then_0`
              (bind _returnvalue_5 (`DataTableFunctionLibrary.GetDataTableColumnAsString` (`self.Data Table`) "Réponse 1"))
              (set `self.Answer1` (`|GetArrayItem` _returnvalue_5 (`self.CurrentQuestion`)))
              (bind _returnvalue_6 (`DataTableFunctionLibrary.GetDataTableColumnAsString` (`self.Data Table`) "Réponse 2"))
              (set `self.Answer2` (`|GetArrayItem` _returnvalue_6 (`self.CurrentQuestion`)))
              (bind _returnvalue_7 (`DataTableFunctionLibrary.GetDataTableColumnAsString` (`self.Data Table`) "Réponse 3"))
              (set `self.Answer3` (`|GetArrayItem` _returnvalue_7 (`self.CurrentQuestion`)))
              (bind _returnvalue_8 (`DataTableFunctionLibrary.GetDataTableColumnAsString` (`self.Data Table`) "Réponse 4"))
              (set `self.Answer4` (`|GetArrayItem` _returnvalue_8 (`self.CurrentQuestion`))))
            (:`then_1`
              (`KismetArrayLibrary.Array_Add` _answers (`self.Answer2`))
              (`KismetArrayLibrary.Array_Add` _answers (`self.Answer3`))
              (`KismetArrayLibrary.Array_Add` _answers (`self.Answer4`))
              (`KismetArrayLibrary.Array_Shuffle` _answers)
              (bind _output_get_2 (set `self.RightAnswerIndex` (`KismetMathLibrary.RandomInteger` 4)))
              (`KismetArrayLibrary.Array_Insert` _answers (`self.Answer1`) _output_get_2))
            (:`then_2`
              (set `/Game/GameplayBlueprints/Cards/WBP_Card.Reponse1_Text` (`KismetTextLibrary.Conv_StringToText` (`|GetArrayItem` (`self.Answers`))) _widgetref_3)
              (set `/Game/GameplayBlueprints/Cards/WBP_Card.Reponse2_Text` (`KismetTextLibrary.Conv_StringToText` (`|GetArrayItem` (`self.Answers`) 1)) _widgetref_3)
              (set `/Game/GameplayBlueprints/Cards/WBP_Card.Reponse3_Text` (`KismetTextLibrary.Conv_StringToText` (`|GetArrayItem` (`self.Answers`) 2)) _widgetref_3)
              (set `/Game/GameplayBlueprints/Cards/WBP_Card.Reponse4_Text` (`KismetTextLibrary.Conv_StringToText` (`|GetArrayItem` (`self.Answers`) 3)) _widgetref_3)
              (`KismetArrayLibrary.Array_Clear` (`self.Answers`)))))))))

(event `self.ReceiveTick`
  (params (DeltaSeconds :type "Float (single-precision)"))
  (bind _widgetref (`self.WidgetRef`))
  (bind _seconds (`/Game/GameplayBlueprints/Cards/WBP_Card.Seconds` _widgetref))
  ;[1 0.8707 0.2011] Timer
  (`KismetSystemLibrary.Delay` 1.0)
  (if (< (`self.Seconds`) 59)
    (bind _result (`/Engine/EditorBlueprintResources/StandardMacros.IncrementInt` (`self.Seconds`))
      (:`  `
        (bind _output_get (set `self.Seconds` _result))
        (`TextBlock.SetText` _seconds (`KismetTextLibrary.Conv_IntToText` _output_get false true 2 2))))
    (else
      (bind _result_2 (`/Engine/EditorBlueprintResources/StandardMacros.IncrementInt` (`self.Minutes`))
        (:`  `
          (bind _output_get_2 (set `self.Minutes` _result_2))
          (set `self.Seconds` 0)
          (`TextBlock.SetText` _seconds (`KismetTextLibrary.Conv_IntToText` 0 false true 2 2))
          (`TextBlock.SetText` (`/Game/GameplayBlueprints/Cards/WBP_Card.Minutes` _widgetref) (`KismetTextLibrary.Conv_IntToText` _output_get_2 false true 2 2)))))))

(fn `UserConstructionScript`)