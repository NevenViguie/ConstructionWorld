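; Generated dynamic mesh actor that uses Geometry Script to build a snow layer over a set of chosen mesh actors.
; GenerateMeshCache merges those meshes in world space and builds a BVH.
; On rebuild, a grid of downward raycasts appends normal-aligned spheres where face normals pass the SnowCoverage test.
; Optional remeshing fuses them through SDF morphology, then smooths, UV-projects, tessellates and texture-displaces before converting to actor space.
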(event `GenerateMeshCache`
  (`|ExecutionSequence`
    (:`then_0`
      ;[1 1 1] Temporary mesh from the array of meshes to add snow to
      (bind _returnvalue (`self.AllocateComputeMesh`))
      (set `self.RaycastMeshActors` _returnvalue)
      (for _array_element (`self.MeshesToAddSnowTo`)
        (bind _returnvalue_2 (`self.AllocateComputeMesh`))
        (bind (_localtoworld _returnvalue_3) (`GeometryScriptLibrary_SceneUtilityFunctions.CopyMeshFromComponent` (`Actor.RootComponent` _array_element) _returnvalue_2 (struct) true null)
          (:`Failure`
            _)
          (:`Success`
            (`GeometryScriptLibrary_MeshBasicEditFunctions.AppendMesh` (`self.RaycastMeshActors`) _returnvalue_3 (struct) false null)))
        (`self.ReleaseComputeMesh` _returnvalue_2)))
    (:`then_1`
      ;[1 1 1] Create BVH and use Raycast to add spheres
      (bind _outputbvh (`GeometryScriptLibrary_MeshSpatial.BuildBVHForMesh` (`self.RaycastMeshActors`) null))
      (set `self.Output BVH` _outputbvh))))

(event `self.OnRebuildGeneratedMesh`
  (params (TargetMesh :type "DynamicMesh Object Reference"))
  (bind _returnvalue (`GeometryScriptLibrary_MeshQueryFunctions.GetMeshBoundingBox` (`self.RaycastMeshActors`)))
  (set `self.Target Mesh` TargetMesh)
  (if (`self.Generate Snow?`)
    (`|ExecutionSequence`
      (:`then_0`
        ;[1 1 1] Create BVH and use Raycast to add spheres
        (for _index (range (+ (`KismetMathLibrary.Round` (/ (- (.x (`.Max` (break `Box` _returnvalue))) (.x (break `Box` _returnvalue))) (`self.GridSpacing`))) 1))
          (for _index_2 (range (+ (`KismetMathLibrary.Round` (/ (- (.y (`.Max` (break `Box` _returnvalue))) (.y (break `Box` _returnvalue))) (`self.GridSpacing`))) 1))
            (bind _hitresult (`GeometryScriptLibrary_MeshSpatial.FindNearestRayIntersectionWithMesh` (`self.RaycastMeshActors`) (`self.Output BVH`) (`KismetMathLibrary.MakeVector` (+ (.x (break `Box` _returnvalue)) (* _index (`self.GridSpacing`))) (+ (.y (break `Box` _returnvalue)) (* _index_2 (`self.GridSpacing`))) (+ (- (.z (`.Max` (break `Box` _returnvalue))) (.z (break `Box` _returnvalue))) 1000.0)) (0.0 0.0 -1.0) (make `GeometryScriptSpatialQueryOptions` 1500.0) null)
              (:`Found`
                (if (`self.UseAltSnowCoverage`)
                  (bind (_bisvalidtriangle _returnvalue_2) (`GeometryScriptLibrary_MeshQueryFunctions.GetTriangleFaceNormal` (`self.RaycastMeshActors`) (`.HitTriangleID` (break `GeometryScriptRayHitResult` _hitresult))))
                  (if (>= (.z _returnvalue_2) (`KismetMathLibrary.Abs` (- (`self.SnowCoverage`) 1.0)))
                    (bind _returnvalue_3 (`KismetMathLibrary.MakeVector` (.x _returnvalue_2) (.y _returnvalue_2) (.z _returnvalue_2)))
                    (`GeometryScriptLibrary_MeshPrimitiveFunctions.AppendSphereBox` (`self.Target Mesh`) (struct) (`KismetMathLibrary.MakeTransform` (`.HitPosition` (break `GeometryScriptRayHitResult` _hitresult)) (`KismetMathLibrary.MakeRotFromZ` _returnvalue_3) (`KismetMathLibrary.MakeVector` 1.0 1.0 (`self.Transform Scale Z`))) (`self.Sphere Radius`) 6 6 6 "Center" null :!label _label))
                  (elif (== _returnvalue_3 (0.0 0.0 1.0) :`ErrorTolerance` (`self.SnowCoverage`))
                    (goto _label))))))))
      (:`then_1`
        ;[1 1 1] Create new voxelised mesh and smooth it + UV & normals
        (if (`self.Remesh`)
          (bind _returnvalue_4 (`GeometryScriptLibrary_MeshVoxelFunctions.ApplyMeshMorphology` (`self.Target Mesh`) (make `GeometryScriptMorphologyOptions` (make `GeometryScript3DGridParameters` "GridCellSize" (`self.Grid Cell Size`)) false (make `GeometryScript3DGridParameters` "GridResolution") "Dilate" (`self.Snow Thickness`)) null))
          (bind _returnvalue_5 (`GeometryScriptLibrary_MeshDeformFunctions.ApplyIterativeSmoothingToMesh` _returnvalue_4 (make `GeometryScriptIterativeMeshSmoothingOptions` (`self.Smooth Iterations`)) null))
          (bind (_returnvalue_min _returnvalue_max) (break `Box` (`GeometryScriptLibrary_MeshQueryFunctions.GetMeshBoundingBox` _returnvalue_5)))
          (bind (_returnvalue_x _returnvalue_y) (`KismetMathLibrary.BreakVector` (- _returnvalue_max _returnvalue_min)))
          (bind _returnvalue_6 (`KismetMathLibrary.FMax` _returnvalue_x _returnvalue_y))
          (bind _returnvalue_7 (`GeometryScriptLibrary_MeshUVFunctions.SetMeshUVsFromPlanarProjection` _returnvalue_5 0 (`KismetMathLibrary.MakeTransform` (0.0 0.0 0.0) (struct) (`KismetMathLibrary.MakeVector` _returnvalue_6 _returnvalue_6 _returnvalue_6)) null))
          (bind _returnvalue_8 (`GeometryScriptLibrary_MeshNormalsFunctions.ComputeTangents` _returnvalue_7 (struct) null))
          (bind _returnvalue_9 (`GeometryScriptLibrary_MeshNormalsFunctions.ComputeSplitNormals` _returnvalue_8 (make `GeometryScriptSplitNormalsOptions` true 80.0) (struct) null))
          (bind _returnvalue_10 (`GeometryScriptLibrary_MeshUVFunctions.ScaleMeshUVs` _returnvalue_9 0 (`self.UV Scale`) (0.5 0.5) null))
          (bind _returnvalue_11 (`GeometryScriptLibrary_MeshUVFunctions.TranslateMeshUVs` _returnvalue_10 0 (`self.UV Offset`) null))
          (`GeometryScriptLibrary_MeshSubdivideFunctions.ApplyPNTessellation` _returnvalue_11 (make `GeometryScriptPNTessellateOptions` true) (`self.Subdivision Amount`) null)))
      (:`then_2`
        ;[1 1 1] Displacementt
        (if (`self.Remesh`)
          (bind _returnvalue_12 (`GeometryScriptLibrary_MeshDeformFunctions.ApplyDisplaceFromTextureMap` (`self.Target Mesh`) (`self.Displacement Texture`) (make `GeometryScriptDisplaceFromTextureOptions` (`self.Displacement Amount`) (1.0 1.0) (0.0 0.0) (`self.Displacement Center`) (`self.Displacement Image Channel`)) 0 null))
          (bind _returnvalue_13 (`GeometryScriptLibrary_MeshNormalsFunctions.ComputeTangents` _returnvalue_12 (struct) null))
          (`GeometryScriptLibrary_MeshNormalsFunctions.ComputeSplitNormals` _returnvalue_13 (make `GeometryScriptSplitNormalsOptions` true 80.0) (struct) null)))
      (:`then_3`
        ;[1 1 1] Reposition the snow on top of original meshes
        (`GeometryScriptLibrary_MeshTransformFunctions.TransformMesh` (`self.Target Mesh`) (`KismetMathLibrary.InvertTransform` (`self.GetTransform`)) null)))))

(fn `UserConstructionScript`)