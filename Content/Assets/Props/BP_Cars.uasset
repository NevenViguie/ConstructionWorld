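; BP_Cars is a prop that sends a single car mesh moving along its local Y axis, repeatedly changing which vehicle it shows.
; After a random startup delay, NextCar picks a hatchback or an SUV, setting rotation for each, plus scale and a random body material for the SUV.
; The CarMovement timeline drives the movement, then a short random delay on completion triggers the next car.
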(event `self.ReceiveBeginPlay`
  (`KismetSystemLibrary.Delay` (+ (* (`KismetMathLibrary.RandomFloat`) 10.0) 7.0))
  (`self.NextCar`))

(event `NextCar`
  (bind _car (`self.Car`))
  (bind _car_2 (`self.Car`))
  (if (< (`KismetMathLibrary.RandomInteger` 5) 3)
    (`StaticMeshComponent.SetStaticMesh` _car "/Game/Assets/Props/SmallCar/MODERNHATCH.MODERNHATCH")
    (`SceneComponent.K2_SetRelativeRotation` (`self.Car`) (struct :`Pitch` 180.0 :`Yaw` 90.0) false false)
    (bind (_direction _y) (`Timeline|CarMovement` :!via `PlayFromStart` :!label _label)
      (:`Update`
        (`SceneComponent.K2_SetRelativeLocation` (`self.Car`) (`KismetMathLibrary.MakeVector` 0.0 _y) false false))
      (:`Finished`
        (`KismetSystemLibrary.Delay` (+ (* (`KismetMathLibrary.RandomFloat`) 2.0) 3.0))
        (`self.NextCar`)))
    (else
      (`StaticMeshComponent.SetStaticMesh` _car "/Game/Assets/Props/SUV/SUV.SUV")
      (`SceneComponent.SetRelativeScale3D` _car_2 (0.11 0.11 0.11))
      (`SceneComponent.K2_SetRelativeRotation` _car_2 (struct :`Yaw` 180.0) false false)
      (`PrimitiveComponent.SetMaterial` _car_2 6 (select `int` (`KismetMathLibrary.RandomInteger` 4) :`0` "/Game/Assets/Props/SUV/dust_body_Grey.dust_body_Grey" :`1` "/Game/Assets/Props/SUV/dust_body_Black.dust_body_Black" :`2` "/Game/Assets/Props/SUV/dust_body_Red.dust_body_Red" :`3` "/Game/Assets/Props/SUV/dust_body_White.dust_body_White" :!type "MaterialInstance Object Reference"))
      (goto _label :!via `PlayFromStart`))))

(fn `UserConstructionScript`)